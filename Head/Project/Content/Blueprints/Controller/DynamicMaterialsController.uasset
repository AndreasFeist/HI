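; Controller that creates and tracks dynamic material instances for mesh slots so their colors can be changed at runtime.
; SetupMaterial picks a source material from a list by ID, creates an instance on the given slot, stores it in a map keyed by slot index and applies the base color.
; SetBaseColor and SetFuzzColor look up that map and set the matching vector parameter when an instance exists.
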(fn `SetBaseColor`
  (params (MaterialID :type Integer) (Color :type "LinearColor Structure"))
  (bind (_value _returnvalue) (`BlueprintMapLibrary.Map_Find` (`self.Materials`) MaterialID))
  (if _returnvalue
    (`MaterialInstanceDynamic.SetVectorParameterValue` _value "BaseColor" Color)))

(fn `SetFuzzColor`
  (params (MeshMaterialID :type Integer) (Color :type "LinearColor Structure"))
  (bind (_value _returnvalue) (`BlueprintMapLibrary.Map_Find` (`self.Materials`) MeshMaterialID))
  (if _returnvalue
    (`MaterialInstanceDynamic.SetVectorParameterValue` _value "FuzzColor" Color)))

(fn `SetupMaterial`
  (params (Materials :type "Array of MaterialInstance Object Reference") (MaterialID :type Integer) (Mesh :type "PrimitiveComponent Object Reference") (MeshMaterialID :type Integer) (Color :type "LinearColor Structure"))
  (bind (_hasitems _selectedmaterial) (`/Game/Blueprints/Controller/AssetsFunctionLibrary.GetSourceMaterial` Materials MaterialID))
  (if _hasitems
    (bind _returnvalue (`PrimitiveComponent.CreateDynamicMaterialInstance` Mesh MeshMaterialID _selectedmaterial))
    (`BlueprintMapLibrary.Map_Add` (`self.Materials`) MeshMaterialID _returnvalue)
    (`self.SetBaseColor` MeshMaterialID Color)))