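; Actor component that highlights what the owner's active camera looks at and lets the owner collect highlighted items.
; Every tick it line-traces along the camera's forward vector, switching highlight meshes to any hit actor with a HighlightComponent and clearing them otherwise.
; InteractWithItem transfers the highlighted actor's Inventory contents to the owner's Inventory through giver and receiver transaction calls, handling only the Collectable highlight type.
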(event `self.ReceiveBeginPlay`
  (bind _returnvalue (`Actor.GetComponentByClass` (`self.GetOwner`) "/Game/Blueprints/Components/Inventory.Inventory_C"))
  (`/Engine/EditorBlueprintResources/StandardMacros.IsValid` _returnvalue
    (:`Is Valid`
      (set `self.OwersInventory` _returnvalue))))

(event `self.ReceiveTick`
  (params (DeltaSeconds :type "Float (single-precision)"))
  (`self.CheckHighlight`))

(fn `CheckHighlight`
  (bind _currenthighlightcomponent (`self.CurrentHighlightComponent`))
  (bind _currenthighlightcomponent_2 (`self.CurrentHighlightComponent`))
  (bind _returnvalue (`Actor.GetComponentByClass` (`self.GetOwner`) "/Game/Blueprints/Controller/CameraController.CameraController_C"))
  (bind _activecamera (`/Game/Blueprints/Controller/CameraController.ActiveCamera` _returnvalue))
  (bind _returnvalue_2 (`SceneComponent.K2_GetComponentLocation` _activecamera))
  (`/Engine/EditorBlueprintResources/StandardMacros.IsValid` _returnvalue
    (:`Is Valid`
      (`/Engine/EditorBlueprintResources/StandardMacros.IsValid` _activecamera
        (:`Is Valid`
          (bind (_outhit _returnvalue_3) (`KismetSystemLibrary.LineTraceSingle` :`Start` _returnvalue_2 :`End` (+ _returnvalue_2 (* (`SceneComponent.GetForwardVector` _activecamera) (`self.HighlightCheckDistance`))) :`TraceChannel` "TraceTypeQuery3" :`DrawTime` 1.0))
          (if _returnvalue_3
            (bind (_result _highlightcomponent) (`self.HasHighlightComponent` (`.HitActor` (`GameplayStatics.BreakHitResult` _outhit))))
            (if _result
              (if (!= (`self.CurrentHighlightComponent`) _highlightcomponent)
                (`/Game/Blueprints/Components/HighlightComponent.ActivateHighlightMeshes` _highlightcomponent)
                (`/Engine/EditorBlueprintResources/StandardMacros.IsValid` _currenthighlightcomponent
                  (:`Is Valid`
                    (`/Game/Blueprints/Components/HighlightComponent.DeactivateHighlightMeshes` _currenthighlightcomponent))
                  (:`Is Not Valid`
                    _))
                (set `self.CurrentHighlightComponent` _highlightcomponent))
              (else
                (`/Engine/EditorBlueprintResources/StandardMacros.IsValid` _currenthighlightcomponent_2 :!label _label
                  (:`Is Valid`
                    (`/Game/Blueprints/Components/HighlightComponent.DeactivateHighlightMeshes` _currenthighlightcomponent_2))
                  (:`Is Not Valid`
                    _))
                (set `self.CurrentHighlightComponent` null)))
            (else
              (goto _label))))))))

(fn `HasHighlightComponent`
  (params (HitActor :type "Actor Object Reference"))
  (returns (Result :type Boolean) (HighlightComponent :type "/Game/Blueprints/Components/HighlightComponent Object Reference"))
  (bind _returnvalue (`Actor.GetComponentByClass` HitActor "/Game/Blueprints/Components/HighlightComponent.HighlightComponent_C"))
  (return (`KismetSystemLibrary.IsValid` _returnvalue) _returnvalue))

(fn `InteractWithItem`
  (bind _currenthighlightcomponent (`self.CurrentHighlightComponent`))
  (bind _owersinventory (`self.OwersInventory`))
  (bind _returnvalue (`Actor.GetComponentByClass` (`self.GetOwner` _currenthighlightcomponent) "/Game/Blueprints/Components/Inventory.Inventory_C"))
  (`/Engine/EditorBlueprintResources/StandardMacros.IsValid` _currenthighlightcomponent
    (:`Is Valid`
      (if (and (`KismetSystemLibrary.IsValid` _returnvalue) (`KismetSystemLibrary.IsValid` _owersinventory))
        (switch `/Game/Blueprints/Components/Lists/HighlightType` (`/Game/Blueprints/Components/HighlightComponent.HighlightType` _currenthighlightcomponent)
          (:`NewEnumerator1`
            (`/Game/Blueprints/Components/HighlightComponent.DeactivateHighlightMeshes` _currenthighlightcomponent)
            (bind _itemstogive (`/Game/Blueprints/Components/Inventory.TransactionGiver` _returnvalue))
            (`/Game/Blueprints/Components/Inventory.TransactionReceiver` _owersinventory _itemstogive)))))))