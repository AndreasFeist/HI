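; Actor component for Characters that caches references to the animation and input variables held by the mesh's Anim Instance.
; On BeginPlay, EnsureInit casts the owner to Character and stops if that fails.
; It then queries the mesh's Anim Instance through message calls and stores the returned AnimationVariables and InputVariables on the component.
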(event `self.ReceiveBeginPlay`
  (`self.EnsureInit`))

(fn `EnsureInit`
  (locals (Character_Temp :type "AnimInstance Object Reference"))
  (bind _character_temp (`local.Character_Temp`))
  (bind _ascharacter (cast `Character` (`self.GetOwner`)))
  (set `local.Character_Temp` (`SkeletalMeshComponent.GetAnimInstance` (`Character.Mesh` _ascharacter)))
  (`|ExecutionSequence`
    (:`then_0`
      (bind _animationvariables (message `/Game/Blueprints/BP_Interfaces/BP_Interface_Animation.GetAnimationVariables` _character_temp))
      (set `self.AnimationVariables` _animationvariables)
      (bind _inputvariables (message `/Game/Blueprints/BP_Interfaces/BP_Interface_Animation.GetInputVariables` _character_temp))
      (set `self.InputVariables` _inputvariables))))