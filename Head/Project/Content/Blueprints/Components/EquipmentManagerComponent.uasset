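; Character component that manages the equipped weapon, spawning it and relaying attack requests to it.
; InitEquipment caches the owning Character, and EquipWeapon spawns a Weapon_Base subclass and snaps it to the socket named by the weapon on the character's mesh.
; AttackWithWeapon calls PrepareAttack on the current weapon, while StopAttackWithWeapon is an empty stub.
; Equipping does not remove any previously held weapon.
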(fn `AttackWithWeapon`
  (bind _equippedweapon (`self.EquippedWeapon`))
  (`/Engine/EditorBlueprintResources/StandardMacros.IsValid` _equippedweapon
    (:`Is Valid`
      (`/Game/Blueprints/Weapons/Weapon_Base.PrepareAttack` _equippedweapon))))

(fn `EquipWeapon`
  (params (WeaponClass :type "Actor Class Reference"))
  (`/Engine/EditorBlueprintResources/StandardMacros.IsValid` (`self.Owner`)
    (:`Is Valid`
      (bind _returnvalue (`|SpawnActorFromClass` WeaponClass (`KismetMathLibrary.MakeTransform` (0.0 0.0 0.0)) "AlwaysSpawn" "OverrideRootScale" null null))
      (bind _asweapon_base (cast `/Game/Blueprints/Weapons/Weapon_Base` _returnvalue))
      (bind _output_get (set `self.EquippedWeapon` _asweapon_base))
      (`Actor.K2_AttachToComponent` _output_get (`Character.Mesh` (`self.Owner`)) (`/Game/Blueprints/Weapons/Weapon_Base.AttachSocket` _output_get) "SnapToTarget" "SnapToTarget" "SnapToTarget" true))))

(fn `InitEquipment`
  (bind _ascharacter (cast `Character` (`self.GetOwner`)))
  (set `self.Owner` _ascharacter))

(fn `StopAttackWithWeapon`)