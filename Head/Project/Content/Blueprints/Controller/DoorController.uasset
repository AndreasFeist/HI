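; Door controller component that animates a door and its grip through opening, open, closing, closed and locked states.
; InteractWithDoor sets the state and toggles ticking, which advances separate door and grip timers to drive relative rotations from vector curves.
; An open door pauses its countdown while the player is near and closes early when they are far.
; The grip presses down again late in closing, and tick disables itself once both current state durations are non-positive.
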(event `self.ReceiveTick`
  (params (DeltaSeconds :type "Float (single-precision)"))
  (`self.HandleActorDoor` DeltaSeconds))

(event `InteractWithDoor`
  (params (NewState :type "/Game/Blueprints/Doors/Lists/DoorStates Enum" :default "NewEnumerator0"))
  (if (and (`|EnumInequality` NewState (`self.DoorState`)) (not (`self.IsComponentTickEnabled`)))
    (set `self.DoorGripState` "NewEnumerator1")
    (bind _output_get (set `self.DoorState` NewState))
    (switch `/Game/Blueprints/Doors/Lists/DoorStates` _output_get
      (:`NewEnumerator0`
        (`self.SetComponentTickEnabled` true :!label _label))
      (:`NewEnumerator2`
        (goto _label))
      (:`NewEnumerator4`
        (`self.SetComponentTickEnabled` false :!label _label_2))
      (:`NewEnumerator3`
        (goto _label_2)))))

(event `UnlockDoor`
  (set `self.DoorState` "NewEnumerator4"))

(event `LockDoor`
  (set `self.DoorState` "NewEnumerator3"))

(fn `DistanceToPlayer`
  (returns (PlayerCloseBy :type Boolean) (PlayerFarAway :type Boolean))
  (bind _returnvalue (`KismetMathLibrary.VSize` (- (`Actor.K2_GetActorLocation` (`GameplayStatics.GetPlayerPawn` 0)) (`Actor.K2_GetActorLocation` (`self.GetOwner`)))))
  (return (<= _returnvalue (`self.PlayerCloseupDistance`)) (>= _returnvalue (`self.PlayerMaxDistance`))))

(fn `HandleActorDoor`
  (params (DeltaSeconds :type "Float (double-precision)"))
  (bind (_playercloseby _playerfaraway) (`self.DistanceToPlayer`))
  (bind _doorstate (`self.DoorState`))
  (bind _returnvalue (+ DeltaSeconds (`self.DoorGripTimer`)))
  (bind _returnvalue_2 (+ (`self.DoorTimer`) DeltaSeconds))
  (bind _returnvalue_3 (/ _returnvalue (select `/Game/Blueprints/Doors/Lists/DoorGripStates` (`self.DoorGripState`) :`NewEnumerator0` (`self.DoorGripUpTme`) :`NewEnumerator1` (`self.DoorGripMoveDownTime`) :`NewEnumerator2` (`self.DoorGripDownTime`) :`NewEnumerator3` (`self.DoorGripMovingUpTime`))))
  (bind _returnvalue_4 (/ _returnvalue_2 (select `/Game/Blueprints/Doors/Lists/DoorStates` (`self.DoorState`) :`NewEnumerator0` (`self.DoorOpeningTime`) :`NewEnumerator1` (`self.DoorOpenTime`) :`NewEnumerator2` (`self.DoorClosingTime`) :`NewEnumerator4` (`self.DoorClosedTime`) :`NewEnumerator3` (`self.DoorLocked`))))
  (`|ExecutionSequence`
    (:`then_0`
      (if (>= _returnvalue_4 1.0)
        (set `self.DoorState` (select `/Game/Blueprints/Doors/Lists/DoorStates` (`self.DoorState`) :`NewEnumerator0` "NewEnumerator1" :`NewEnumerator1` "NewEnumerator2" :`NewEnumerator2` "NewEnumerator4" :`NewEnumerator4` "NewEnumerator4" :`NewEnumerator3` "NewEnumerator3" :!type "/Game/Blueprints/Doors/Lists/DoorStates Enum"))
        (set `self.DoorTimer` 0.0)
        (elif (not (and (`|EnumEquality` "NewEnumerator1" _doorstate) _playercloseby))
          (set `self.DoorTimer` _returnvalue_2)
          (if (and _playerfaraway (`|EnumEquality` _doorstate "NewEnumerator1"))
            (set `self.DoorState` "NewEnumerator2")
            (set `self.DoorTimer` 0.0)
            (else
              (`self.HandleDoor` (`self.DoorState`) _returnvalue_4))))))
    (:`then_1`
      (if (>= _returnvalue_3 1.0)
        (set `self.DoorGripState` (select `/Game/Blueprints/Doors/Lists/DoorGripStates` (`self.DoorGripState`) :`NewEnumerator0` "NewEnumerator1" :`NewEnumerator1` "NewEnumerator2" :`NewEnumerator2` "NewEnumerator3" :`NewEnumerator3` "NewEnumerator0" :!type "/Game/Blueprints/Doors/Lists/DoorGripStates Enum"))
        (set `self.DoorGripTimer` 0.0)
        (else
          (set `self.DoorGripTimer` _returnvalue)
          (if (and (`|EnumEquality` (`self.DoorState`) "NewEnumerator2") (>= _returnvalue_4 0.75) (`|EnumEquality` (`self.DoorGripState`) "NewEnumerator0"))
            (set `self.DoorGripState` "NewEnumerator1")
            (set `self.DoorGripTimer` 0.0)
            (else
              (`self.HandleGrip` _returnvalue_3 (`self.DoorGripState`)))))))
    (:`then_2`
      (if (and (<= (select `/Game/Blueprints/Doors/Lists/DoorStates` (`self.DoorState`) :`NewEnumerator0` (`self.DoorOpeningTime`) :`NewEnumerator1` (`self.DoorOpenTime`) :`NewEnumerator2` (`self.DoorClosingTime`) :`NewEnumerator4` (`self.DoorClosedTime`) :`NewEnumerator3` (`self.DoorLocked`)) 0.0) (<= (select `/Game/Blueprints/Doors/Lists/DoorGripStates` (`self.DoorGripState`) :`NewEnumerator0` (`self.DoorGripUpTme`) :`NewEnumerator1` (`self.DoorGripMoveDownTime`) :`NewEnumerator2` (`self.DoorGripDownTime`) :`NewEnumerator3` (`self.DoorGripMovingUpTime`)) 0.0))
        (set `self.DoorGripTimer` 0.0)
        (set `self.DoorTimer` 0.0)
        (`self.SetComponentTickEnabled` false)))))

(fn `HandleDoor`
  (params (DoorState :type "/Game/Blueprints/Doors/Lists/DoorStates Enum" :default "NewEnumerator0") (Time :type "Float (double-precision)"))
  (bind _doorclosecurve (`self.DoorCloseCurve`))
  (bind _door (`self.Door`))
  (bind _dooropencurve (`self.DoorOpenCurve`))
  (if (and (`KismetSystemLibrary.IsValid` _door) (`KismetSystemLibrary.IsValid` (`self.DoorOpenCurve`)) (`KismetSystemLibrary.IsValid` (`self.DoorCloseCurve`)))
    (`SceneComponent.K2_SetRelativeRotation` _door (`KismetMathLibrary.MakeRotator` (.x (`CurveVector.GetVectorValue` (select `/Game/Blueprints/Doors/Lists/DoorStates` DoorState :`NewEnumerator0` _dooropencurve :`NewEnumerator1` _doorclosecurve :`NewEnumerator2` _doorclosecurve :`NewEnumerator4` _dooropencurve :`NewEnumerator3` _doorclosecurve) (select `/Game/Blueprints/Doors/Lists/DoorStates` DoorState :`NewEnumerator0` Time :`NewEnumerator2` Time :`NewEnumerator3` 1.0))) (.y (`CurveVector.GetVectorValue` (select `/Game/Blueprints/Doors/Lists/DoorStates` DoorState :`NewEnumerator0` _dooropencurve :`NewEnumerator1` _doorclosecurve :`NewEnumerator2` _doorclosecurve :`NewEnumerator4` _dooropencurve :`NewEnumerator3` _doorclosecurve) (select `/Game/Blueprints/Doors/Lists/DoorStates` DoorState :`NewEnumerator0` Time :`NewEnumerator2` Time :`NewEnumerator3` 1.0))) (.z (`CurveVector.GetVectorValue` (select `/Game/Blueprints/Doors/Lists/DoorStates` DoorState :`NewEnumerator0` _dooropencurve :`NewEnumerator1` _doorclosecurve :`NewEnumerator2` _doorclosecurve :`NewEnumerator4` _dooropencurve :`NewEnumerator3` _doorclosecurve) (select `/Game/Blueprints/Doors/Lists/DoorStates` DoorState :`NewEnumerator0` Time :`NewEnumerator2` Time :`NewEnumerator3` 1.0)))) false false)
    (return)))

(fn `HandleGrip`
  (params (Time :type "Float (double-precision)") (GripState :type "/Game/Blueprints/Doors/Lists/DoorGripStates Enum" :default "NewEnumerator0"))
  (bind _doorgrip (`self.DoorGrip`))
  (if (and (`KismetSystemLibrary.IsValid` _doorgrip) (`KismetSystemLibrary.IsValid` (`self.DoorGripCurve`)))
    (`SceneComponent.K2_SetRelativeRotation` _doorgrip (`KismetMathLibrary.MakeRotator` (.x (`CurveVector.GetVectorValue` (`self.DoorGripCurve`) (select `/Game/Blueprints/Doors/Lists/DoorGripStates` GripState :`NewEnumerator1` Time :`NewEnumerator2` 1.0 :`NewEnumerator3` (- 1.0 Time)))) (.y (`CurveVector.GetVectorValue` (`self.DoorGripCurve`) (select `/Game/Blueprints/Doors/Lists/DoorGripStates` GripState :`NewEnumerator1` Time :`NewEnumerator2` 1.0 :`NewEnumerator3` (- 1.0 Time)))) (.z (`CurveVector.GetVectorValue` (`self.DoorGripCurve`) (select `/Game/Blueprints/Doors/Lists/DoorGripStates` GripState :`NewEnumerator1` Time :`NewEnumerator2` 1.0 :`NewEnumerator3` (- 1.0 Time))))) false false)))

(fn `InitializeController`
  (params (Door :type "StaticMeshComponent Object Reference") (DoorOpenCurve :type "CurveVector Object Reference") (DoorCloseCurve :type "CurveVector Object Reference") (DoorRotation :type "Float (double-precision)") (DoorGrip :type "StaticMeshComponent Object Reference") (DoorGripCurve :type "CurveVector Object Reference") (GripRotation :type "Float (double-precision)"))
  (set `self.Door` Door)
  (set `self.DoorOpenCurve` DoorOpenCurve)
  (set `self.DoorCloseCurve` DoorCloseCurve)
  (set `self.DoorGrip` DoorGrip)
  (set `self.DoorGripCurve` DoorGripCurve)
  (`self.HandleDoor` "NewEnumerator2" (- 1.0 DoorRotation))
  (`self.HandleGrip` GripRotation "NewEnumerator1"))

(fn `SetupDistances`
  (params (InteractionRadius :type "Float (double-precision)"))
  (set `self.PlayerMaxDistance` (* InteractionRadius 2.0))
  (set `self.PlayerCloseupDistance` (/ InteractionRadius 2.0)))