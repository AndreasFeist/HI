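; Actor component that toggles highlighting on its owning actor through custom depth and stencil rendering.
; Activation enables custom depth on all of the owner's primitive components and sets a stencil value chosen by HighlightType, distinguishing default, collectable, chest and character highlights.
; Deactivation disables custom depth on those components and clears the stencil.
; The event graph holds no active logic, so both functions rely on external calls.
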(fn `ActivateHighlightMeshes`
  (bind _returnvalue (`Actor.K2_GetComponentsByClass` (`self.GetOwner`) "/Script/Engine.PrimitiveComponent"))
  (`PrimitiveComponent.SetRenderCustomDepth` _returnvalue true)
  (`PrimitiveComponent.SetCustomDepthStencilValue` _returnvalue (select `/Game/Blueprints/Components/Lists/HighlightType` (`self.HighlightType`) :`NewEnumerator0` 9 :`NewEnumerator1` 10 :`NewEnumerator2` 11 :`NewEnumerator3` 12)))

(fn `DeactivateHighlightMeshes`
  (bind _returnvalue (`Actor.K2_GetComponentsByClass` (`self.GetOwner`) "/Script/Engine.PrimitiveComponent"))
  (`PrimitiveComponent.SetRenderCustomDepth` _returnvalue false)
  (`PrimitiveComponent.SetCustomDepthStencilValue` _returnvalue 0))