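; A Blueprint function library of safe list lookups for static meshes, source materials and door frame structs.
; Each function takes a list and an ID, returns the matching entry, and falls back to index 0 when the ID exceeds the last index.
; All three report whether the list has items, and the mesh lookup also returns the resolved ID, or 0 for an empty list.
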(fn `GetDoorStruct`
  (params (FramesList :type "Array of /Game/Blueprints/Doors/Lists/DoorSStruct Structure") (DoorFrameID :type Integer))
  (returns (HasItems :type Boolean) (Frame :type "/Game/Blueprints/Doors/Lists/DoorSStruct Structure"))
  (bind _returnvalue (> (`KismetArrayLibrary.Array_Length` FramesList) 0))
  (if _returnvalue
    (return _returnvalue (`|GetArrayItem` FramesList (`KismetMathLibrary.SelectInt` DoorFrameID 0 (<= DoorFrameID (`KismetArrayLibrary.Array_LastIndex` FramesList)))))
    (else
      (return _returnvalue))))

(fn `GetSourceMaterial`
  (params (MaterialsList :type "Array of MaterialInstance Object Reference (by ref)") (CurrentID :type Integer))
  (returns (HasItems :type Boolean) (SelectedMaterial :type "MaterialInstance Object Reference"))
  (bind _returnvalue (> (`KismetArrayLibrary.Array_Length` MaterialsList) 0))
  (if _returnvalue
    (return _returnvalue (`|GetArrayItem` MaterialsList (`KismetMathLibrary.SelectInt` CurrentID 0 (<= CurrentID (`KismetArrayLibrary.Array_LastIndex` MaterialsList)))))
    (else
      (return _returnvalue null))))

(fn `GetStaticMesh`
  (params (AssetList :type "Array of StaticMesh Object Reference (by ref)") (CurrentID :type Integer))
  (returns (HasItems :type Boolean) (Mesh :type "StaticMesh Object Reference") (ID :type Integer))
  (bind _returnvalue (> (`KismetArrayLibrary.Array_Length` AssetList) 0))
  (bind _returnvalue_2 (`KismetMathLibrary.SelectInt` CurrentID 0 (<= CurrentID (`KismetArrayLibrary.Array_LastIndex` AssetList))))
  (if _returnvalue
    (return _returnvalue (`|GetArrayItem` AssetList _returnvalue_2) _returnvalue_2)
    (else
      (return _returnvalue null 0))))