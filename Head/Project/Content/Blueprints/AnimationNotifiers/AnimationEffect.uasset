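; AnimationEffect is an effect actor that bundles the visual, audio, haptic and decal feedback for one selected animation effect.
; Its construction script adds particle system, audio, force feedback and decal components.
; Each component takes its asset from the matching AnimationEffects collection, with SelectedEffect as the shared lookup key.
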(fn `UserConstructionScript`
  (bind _selectedeffect (`self.SelectedEffect`))
  (bind (_particlefx _soundfx _forcefeedbackfx _decalfx) (break `/Game/Blueprints/AnimationNotifiers/Lists/AnimEvent_Outputs` (`self.AnimationEffects`)))
  (`|ExecutionSequence`
    (:`then_0`
      (bind _returnvalue (`AddComponent|NODE_AddParticleSystemComponent-0`))
      (`ParticleSystemComponent.SetTemplate` _returnvalue (`|GetArrayItem` _particlefx _selectedeffect)))
    (:`then_1`
      (bind _returnvalue_2 (`AddComponent|NODE_AddAudioComponent-0`))
      (`AudioComponent.SetSound` _returnvalue_2 (`|GetArrayItem` _soundfx _selectedeffect)))
    (:`then_2`
      (bind _returnvalue_3 (`AddComponent|NODE_AddForceFeedbackComponent-0`))
      (`ForceFeedbackComponent.SetForceFeedbackEffect` _returnvalue_3 (`|GetArrayItem` _forcefeedbackfx _selectedeffect)))
    (:`then_3`
      (bind _returnvalue_4 (`AddComponent|NODE_AddDecalComponent-0`))
      (`DecalComponent.SetDecalMaterial` _returnvalue_4 (`|GetArrayItem` _decalfx _selectedeffect)))))