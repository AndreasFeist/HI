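; Base door actor that assembles a configurable door in the construction script and triggers interaction when the player pawn overlaps it.
; Frame, door, lock and grip are built as a chain, socket-snapped with meshes and materials picked by ID through DynamicMaterialsController components.
; Only swing doors return door data, chosen by hinge side.
; DoorController receives meshes, curves, rotations and the sphere radius to handle interaction.
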(event `self.ReceiveActorBeginOverlap`
  (params (OtherActor :type "Actor Object Reference"))
  (if (== OtherActor (`GameplayStatics.GetPlayerPawn` 0))
    (`/Game/Blueprints/Controller/DoorController.InteractWithDoor` (`self.DoorController`) "NewEnumerator0")))

(fn `GetDoor`
  (returns (ReturnValue :type "/Game/Blueprints/Doors/Lists/DoorSStruct Structure"))
  (return (select `/Game/Blueprints/Doors/Lists/DoorType` (`self.DoorType`) :`NewEnumerator1` (`self.GetSwingDoor`))))

(fn `GetSwingDoor`
  (returns (List :type "/Game/Blueprints/Doors/Lists/DoorSStruct Structure (by ref)"))
  (bind _doorid (`self.DoorID`))
  (bind _doorrightlist (`self.DoorRightList`))
  (bind _doorleftlist (`self.DoorLeftList`))
  (bind _dooruplist (`self.DoorUpList`))
  (bind _doordownlist (`self.DoorDownList`))
  (bind _doorsstruct (make `/Game/Blueprints/Doors/Lists/DoorSStruct` null (`|MakeArray`)))
  (return (select `/Game/Blueprints/Doors/Lists/DoorHinges` (`self.DoorHinges`) :`NewEnumerator1` (select `bool` (== (`KismetArrayLibrary.Array_Length` _doorleftlist) 0) :`false` (`|GetArrayItem` _doorleftlist _doorid) :`true` _doorsstruct) :`NewEnumerator0` (select `bool` (== (`KismetArrayLibrary.Array_Length` _doorrightlist) 0) :`false` (`|GetArrayItem` _doorrightlist _doorid) :`true` _doorsstruct) :`NewEnumerator5` (select `bool` (== (`KismetArrayLibrary.Array_Length` _dooruplist) 0) :`false` (`|GetArrayItem` _dooruplist _doorid) :`true` _doorsstruct) :`NewEnumerator6` (select `bool` (== (`KismetArrayLibrary.Array_Length` _doordownlist) 0) :`false` (`|GetArrayItem` _doordownlist _doorid) :`true` _doorsstruct))))

(fn `SetupAdditionalMeshes`
  (if (`self.UseAdditionalMeshes`)
    (bind _returnvalue (`AddComponent|NODE_AddStaticMeshComponent-0`))
    (`StaticMeshComponent.SetStaticMesh` _returnvalue (`self.AdditionalMesh`))))

(fn `SetupDoor`
  (returns (MeshSet :type Boolean))
  (bind _door (`self.Door`))
  (bind (_mesh _materials) (break `/Game/Blueprints/Doors/Lists/DoorSStruct` (`self.GetDoor`)))
  (`SceneComponent.K2_AttachToComponent` (`self.Door`) (`self.DoorFrame`) (select `/Game/Blueprints/Doors/Lists/DoorHinges` (`self.DoorHinges`) :`NewEnumerator1` "DoorLeft" :`NewEnumerator0` "DoorRight" :`NewEnumerator5` "DoorUp" :`NewEnumerator6` "DoorDown" :!type "Name") "SnapToTarget" "SnapToTarget" "SnapToTarget" true)
  (bind _returnvalue (`StaticMeshComponent.SetStaticMesh` _door _mesh))
  (`/Game/Blueprints/Controller/DynamicMaterialsController.SetupMaterial` (`self.DynamicMaterialsController_Door`) _materials (`self.DoorMaterialID`) _door 0 (`self.DoorColor`))
  (return _returnvalue))

(fn `SetupDoorFrame`
  (returns (MeshSet :type Boolean))
  (bind _doorframe (`self.DoorFrame`))
  (bind (_hasitems _frame) (`/Game/Blueprints/Controller/AssetsFunctionLibrary.GetDoorStruct` (`self.DoorFramesList`) (`self.DoorFrameID`)))
  (bind (_mesh _materials) (break `/Game/Blueprints/Doors/Lists/DoorSStruct` _frame))
  (if _hasitems
    (bind _returnvalue (`StaticMeshComponent.SetStaticMesh` _doorframe _mesh))
    (`/Game/Blueprints/Controller/DynamicMaterialsController.SetupMaterial` (`self.DynamicMaterialsController_Frame`) _materials (`self.DoorFrameMaterialID`) _doorframe 0 (`self.DoorFrameColor`))
    (return _returnvalue)))

(fn `SetupDoorGrip`
  (returns (MeshSet :type Boolean))
  (bind _doorgrip (`self.DoorGrip`))
  (bind (_hasitems _frame) (`/Game/Blueprints/Controller/AssetsFunctionLibrary.GetDoorStruct` (`self.DoorGripList`) (`self.DoorGripID`)))
  (bind (_mesh _materials) (break `/Game/Blueprints/Doors/Lists/DoorSStruct` _frame))
  (`SceneComponent.K2_AttachToComponent` (`self.DoorGrip`) (`self.DoorLock`) "DoorGrip" "SnapToTarget" "SnapToTarget" "SnapToTarget" true)
  (if _hasitems
    (bind _returnvalue (`StaticMeshComponent.SetStaticMesh` _doorgrip _mesh))
    (`/Game/Blueprints/Controller/DynamicMaterialsController.SetupMaterial` (`self.DynamicMaterialsController_Grip`) _materials (`self.DoorGripMaterialID`) _doorgrip 0 (`self.DoorGripColor`))
    (return _returnvalue)))

(fn `SetupDoorLock`
  (returns (MeshSet :type Boolean))
  (bind _doorlock (`self.DoorLock`))
  (bind (_hasitems _frame) (`/Game/Blueprints/Controller/AssetsFunctionLibrary.GetDoorStruct` (`self.DoorLockList`) (`self.DoorLockID`)))
  (bind (_mesh _materials) (break `/Game/Blueprints/Doors/Lists/DoorSStruct` _frame))
  (`SceneComponent.K2_AttachToComponent` (`self.DoorLock`) (`self.Door`) "DoorLock" "SnapToTarget" "SnapToTarget" "SnapToTarget" true)
  (if _hasitems
    (bind _returnvalue (`StaticMeshComponent.SetStaticMesh` _doorlock _mesh))
    (`/Game/Blueprints/Controller/DynamicMaterialsController.SetupMaterial` (`self.DynamicMaterialsController_Lock`) _materials (`self.DoorLockMaterialID`) _doorlock 0 (`self.DoorLockColor`))
    (return _returnvalue)))

(fn `SetupInteraction`
  (bind _sphere (`self.Sphere`))
  (`/Game/Blueprints/Controller/DoorController.InitializeController` (`self.DoorController`) (`self.Door`) (`self.DoorOpenCurve`) (`self.DoorCloseCuve`) (`self.DoorRotation`) (`self.DoorGrip`) (`self.DoorGripCurve`) (`self.GripRotation`))
  (`SphereComponent.SetSphereRadius` _sphere (`self.DoorSphereRadius`) true)
  (`SceneComponent.K2_SetRelativeLocation` _sphere (`KismetMathLibrary.MakeVector` 0.0 0.0 (`.SphereRadius` (`KismetSystemLibrary.GetComponentBounds` (`self.Door`)))) false false)
  (`/Game/Blueprints/Controller/DoorController.SetupDistances` (`self.DoorController`) (`self.DoorSphereRadius`)))

(fn `UserConstructionScript`
  (`|ExecutionSequence`
    (:`then_0`
      (bind _meshset (`self.SetupDoorFrame`))
      (if _meshset
        (bind _meshset_2 (`self.SetupDoor`))
        (if _meshset_2
          (bind _meshset_3 (`self.SetupDoorLock`))
          (if _meshset_3
            (`self.SetupDoorGrip`)
            (`self.SetupAdditionalMeshes`)))))
    (:`then_1`
      (`self.SetupInteraction`))))