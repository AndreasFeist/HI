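; Camera controller component that switches a character between first-person and third-person views and swaps the third-person shoulder side.
; InitCameras stores the supplied cameras, boom and mesh sets; perspective toggling activates one camera and sets owner-no-see on the meshes to match.
; Shoulder toggling, allowed only in third person, flips direction and enables tick, which moves the boom along a vector curve until it reaches either end, then disables tick.
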(event `self.ReceiveTick`
  (params (DeltaSeconds :type "Float (single-precision)"))
  (`self.CameraSideShift` DeltaSeconds))

(fn `CameraPerspectiveToggle`
  (bind _tp_camera (`self.TP_Camera`))
  (bind _isinfp (`self.IsInFP`))
  (bind _fp_camera (`self.FP_Camera`))
  (if _isinfp
    (`self.SetActive` (`self.FP_Camera`) false false)
    (`self.SetActive` _tp_camera true false)
    (`self.SetActiveCamera` _tp_camera)
    (`PrimitiveComponent.SetOwnerNoSee` (`self.FPMeshes`) true)
    (`PrimitiveComponent.SetOwnerNoSee` (`self.TPMeshes`) false)
    (else
      (`self.SetActive` _fp_camera true false)
      (`self.SetActive` (`self.TP_Camera`) false false)
      (`self.SetActiveCamera` _fp_camera)
      (`PrimitiveComponent.SetOwnerNoSee` (`self.FPMeshes`) false)
      (`PrimitiveComponent.SetOwnerNoSee` (`self.TPMeshes`) true)))
  (set `self.IsInFP` (not _isinfp)))

(fn `CameraShoulderPerspectiveToggle`
  (if (== (`self.ActiveCamera`) (`self.TP_Camera`))
    (`self.SetComponentTickEnabled` true)
    (if (== (`self.IsLeft`) 1)
      (set `self.IsLeft` -1)
      (else
        (set `self.IsLeft` 1)))))

(fn `CameraSideShift`
  (params (TimeDelta :type "Float (double-precision)"))
  (bind _transitiontime (`self.TransitionTime`))
  (bind _output_get (set `self.TransitionTime` (+ (* (* (`self.IsLeft`) TimeDelta) (`self.TransitionSpeed`)) (`self.TransitionTime`))))
  (`SceneComponent.K2_SetRelativeLocation` (`self.TP_CameraBoom`) (`CurveVector.GetVectorValue` (`self.CameraBoomCurve`) _output_get) false false)
  (if (>= _transitiontime 1.0)
    (set `self.TransitionTime` 1.0)
    (`self.SetComponentTickEnabled` false :!label _label)
    (elif (<= _transitiontime -1.0)
      (set `self.TransitionTime` -1.0)
      (goto _label))))

(fn `InitCameras`
  (params (FP_Camera :type "CameraComponent Object Reference") (FP_Meshes :type "Array of PrimitiveComponent Object Reference") (TP_CameraBoom :type "SpringArmComponent Object Reference") (TP_Camera :type "CameraComponent Object Reference") (TP_Meshes :type "Array of PrimitiveComponent Object Reference"))
  (`/Engine/EditorBlueprintResources/StandardMacros.IsValid` FP_Camera
    (:`Is Valid`
      (set `self.FP_Camera` FP_Camera))
    (:`Is Not Valid`
      _))
  (if (and (> (`KismetArrayLibrary.Array_Length` FP_Meshes) 0) (`KismetSystemLibrary.IsValid` (`|GetArrayItem` FP_Meshes)))
    (set `self.FPMeshes` FP_Meshes))
  (`/Engine/EditorBlueprintResources/StandardMacros.IsValid` TP_CameraBoom
    (:`Is Valid`
      (set `self.TP_CameraBoom` TP_CameraBoom))
    (:`Is Not Valid`
      _))
  (`/Engine/EditorBlueprintResources/StandardMacros.IsValid` TP_Camera
    (:`Is Valid`
      (set `self.TP_Camera` TP_Camera))
    (:`Is Not Valid`
      _))
  (if (and (> (`KismetArrayLibrary.Array_Length` TP_Meshes) 0) (`KismetSystemLibrary.IsValid` (`|GetArrayItem` TP_Meshes)))
    (set `self.TPMeshes` TP_Meshes)))

(fn `SetActiveCamera`
  (params (NewActiveCamera :type "CameraComponent Object Reference"))
  (set `self.ActiveCamera` NewActiveCamera))