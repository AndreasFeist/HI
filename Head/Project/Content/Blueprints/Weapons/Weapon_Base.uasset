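; Base weapon Blueprint that provides a line-trace attack.
; PrepareAttack calls Attack directly, which runs a multi line trace on the Visibility channel from the AttackDirection component along its forward vector for AttackDistance.
; The trace is debug-drawn for a duration, and its hit results are not used, so no damage or effects are applied here.
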(fn `Attack`
  (bind _attackdirection (`self.AttackDirection`))
  (bind _returnvalue (`SceneComponent.K2_GetComponentLocation` _attackdirection))
  (`KismetSystemLibrary.LineTraceMulti` :`Start` _returnvalue :`End` (+ _returnvalue (* (`KismetMathLibrary.Normal` (`SceneComponent.GetForwardVector` _attackdirection)) (`self.AttackDistance`))) :`TraceChannel` "TraceTypeQuery1" :`DrawDebugType` "ForDuration"))

(fn `PrepareAttack`
  (`self.Attack`))

(fn `UserConstructionScript`
  (`parent.UserConstructionScript`))