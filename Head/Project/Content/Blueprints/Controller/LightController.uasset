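; LightController is a Blueprint helper that attaches a light component to a parent's "Light" socket and configures it from a LightProperties struct.
; SetupLight casts the light by type and calls SetPointLight or SetSpotLight to apply source size, attenuation, intensity, color, shadows and light function, plus cone angles for spots.
; The spot branch leaves SetSpotLight's SpotLight input unconnected, and the directional branch only casts.
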(fn `SetPointLight`
  (params (Light :type "PointLightComponent Object Reference") (LightProperties :type "/Game/Blueprints/Controller/Lists/LightProperties Structure (by ref)"))
  (bind ((`SourceRadius_2_7A69F7E94413DDC4D73FF8B896DE115B` _sourceradius) (`SourceLength_4_48FCBC2841803AF9682E6CAAD17C0CFC` _sourcelength) (`AttenuationRadius_12_8989E37F4A821DF0ED99D3A8ECE787E9` _attenuationradius) (`LightIntensty_20_D1CFBB004ABE7D285E39249286D6A537` _lightintensty) (`LightColor_11_53A285124BB976E44572AF8D5E22F861` _lightcolor) (`CastShadows_15_E851EC0D4EECF42B4EB083AC9BA90B02` _castshadows) (`LightFunction_17_2C7966CF474B807DDFF73FB108FA4166` _lightfunction)) (break `/Game/Blueprints/Controller/Lists/LightProperties` LightProperties))
  (`PointLightComponent.SetSourceRadius` Light _sourceradius)
  (`PointLightComponent.SetSourceLength` Light _sourcelength)
  (`PointLightComponent.SetAttenuationRadius` Light _attenuationradius)
  (`LightComponent.SetIntensity` Light _lightintensty)
  (`LightComponent.SetLightColor` Light _lightcolor true)
  (`LightComponentBase.SetCastShadows` Light _castshadows)
  (`LightComponent.SetLightFunctionMaterial` Light _lightfunction))

(fn `SetSpotLight`
  (params (SpotLight :type "SpotLightComponent Object Reference") (LightProperties :type "/Game/Blueprints/Controller/Lists/LightProperties Structure (by ref)"))
  (bind (_sourceradius _sourcelength _innerconeangle _outerconeangle _attenuationradius _lightintensty _lightcolor _castshadows _lightfunction) (break `/Game/Blueprints/Controller/Lists/LightProperties` LightProperties))
  (`PointLightComponent.SetSourceRadius` SpotLight _sourceradius)
  (`PointLightComponent.SetSourceLength` SpotLight _sourcelength)
  (`SpotLightComponent.SetInnerConeAngle` SpotLight _innerconeangle)
  (`SpotLightComponent.SetOuterConeAngle` SpotLight _outerconeangle)
  (`PointLightComponent.SetAttenuationRadius` SpotLight _attenuationradius)
  (`LightComponent.SetIntensity` SpotLight _lightintensty)
  (`LightComponent.SetLightColor` SpotLight _lightcolor true)
  (`LightComponentBase.SetCastShadows` SpotLight _castshadows)
  (`LightComponent.SetLightFunctionMaterial` SpotLight _lightfunction))

(fn `SetupLight`
  (params (Light :type "LightComponent Object Reference") (AttachComponent :type "PrimitiveComponent Object Reference") (LightProperties :type "/Game/Blueprints/Controller/Lists/LightProperties Structure (by ref)"))
  (`SceneComponent.K2_AttachToComponent` Light AttachComponent "Light" "SnapToTarget" "SnapToTarget" "SnapToTarget" true)
  (`|ExecutionSequence`
    (:`then_0`
      (bind _aspoint_light_component (cast `PointLightComponent` Light))
      (`self.SetPointLight` _aspoint_light_component LightProperties))
    (:`then_1`
      (cast `SpotLightComponent` Light)
      (`self.SetSpotLight` null LightProperties))
    (:`then_2`
      (cast `DirectionalLightComponent` Light))))