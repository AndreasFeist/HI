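; Inventory component that holds item stacks and handles giving and receiving them, with collectable and replenishing owner types.
; TransactionGiver deducts ItemsToGive, or all Items by default, then destroys an emptied Collectable or enables Tick on a replenishing one.
; Tick is meant to add RechargeResources after RechargeTime, then switch itself off.
; As wired, RechargeTimer never accumulates, ReceiveResources' length check never passes, and the replenish branch returns no items.
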(event `self.ReceiveTick`
  (params (DeltaSeconds :type "Float (single-precision)"))
  (if (`self.ChargeUp` DeltaSeconds)
    (`self.RechargeInventory`)
    (`self.SetComponentTickEnabled` false)))

(fn `ChargeUp`
  (params (TimeDelta :type "Float (double-precision)"))
  (returns (ChargedUp :type Boolean))
  (if (>= (+ TimeDelta (`self.RechargeTimer`)) (`self.RechargeTime`))
    (set `self.RechargeTimer` 0.0)
    (return true)
    (else
      (return false))))

(fn `CleanupGiver`
  (if (== 0 (`KismetArrayLibrary.Array_Length` (`self.Items`)))
    (`Actor.K2_DestroyActor` (`self.GetOwner` self))))

(fn `GetItemsToGive`
  (returns (ItemsToGive :type "Array of /Game/Blueprints/Components/Lists/Item Structure"))
  (bind _itemstogive (`self.ItemsToGive`))
  (return (select `bool` (> (`KismetArrayLibrary.Array_Length` _itemstogive) 0) :`false` (`self.Items`) :`true` _itemstogive)))

(fn `GiveResources`
  (returns (ItemsToGive :type "Array of /Game/Blueprints/Components/Lists/Item Structure"))
  (bind _itemstogive (`self.GetItemsToGive`))
  (bind _items (`self.Items`))
  (for _array_element _itemstogive
    (bind _returnvalue (`KismetArrayLibrary.Array_Find` _items _array_element))
    (bind _returnvalue_2 (- (`.NumberOfItems_2_E4AC7DFC457F33FD6A1A5580F7E8212C` (break `/Game/Blueprints/Components/Lists/Item` (`|GetArrayItem` _items _returnvalue))) (`.NumberOfItems_2_E4AC7DFC457F33FD6A1A5580F7E8212C` (break `/Game/Blueprints/Components/Lists/Item` _array_element))))
    (if (> _returnvalue_2 0)
      (setmembers `/Game/Blueprints/Components/Lists/Item` :`StructRef` (`|GetArrayItem` (`self.Items`) _returnvalue) :`NumberOfItems` _returnvalue_2)
      (else
        (`KismetArrayLibrary.Array_Remove` (`self.Items`) _returnvalue))))
  (return _itemstogive))

(fn `ReceiveResources`
  (params (ReceivedItems :type "Array of /Game/Blueprints/Components/Lists/Item Structure"))
  (bind _items (`self.Items`))
  (if (> 0 (`KismetArrayLibrary.Array_Length` ReceivedItems))
    (for _array_element ReceivedItems
      (bind _returnvalue (`KismetArrayLibrary.Array_Find` (`self.Items`) _array_element))
      (if (>= _returnvalue 0)
        (bind _output (`|GetArrayItem` _items _returnvalue))
        (setmembers `/Game/Blueprints/Components/Lists/Item` :`StructRef` _output :`NumberOfItems` (+ (`.NumberOfItems_2_E4AC7DFC457F33FD6A1A5580F7E8212C` (break `/Game/Blueprints/Components/Lists/Item` _output)) (`.NumberOfItems_2_E4AC7DFC457F33FD6A1A5580F7E8212C` (break `/Game/Blueprints/Components/Lists/Item` _array_element))))
        (else
          (`KismetArrayLibrary.Array_Add` _items _array_element))))))

(fn `RechargeInventory`
  (bind _items (`self.Items`))
  (for _array_element (`self.RechargeResources`)
    (bind _returnvalue (`KismetArrayLibrary.Array_Find` (`self.Items`) _array_element))
    (if (>= _returnvalue 0)
      (bind _output (`|GetArrayItem` _items _returnvalue))
      (setmembers `/Game/Blueprints/Components/Lists/Item` :`StructRef` _output :`NumberOfItems` (+ (`.NumberOfItems_2_E4AC7DFC457F33FD6A1A5580F7E8212C` (break `/Game/Blueprints/Components/Lists/Item` _output)) (`.NumberOfItems_2_E4AC7DFC457F33FD6A1A5580F7E8212C` (break `/Game/Blueprints/Components/Lists/Item` _array_element))))
      (else
        (`KismetArrayLibrary.Array_Add` _items _array_element)))))

(fn `ReplenishGiver`
  (`self.SetComponentTickEnabled` true))

(fn `TransactionGiver`
  (returns (ItemsToGive :type "Array of /Game/Blueprints/Components/Lists/Item Structure"))
  (bind _itemstogive (`self.GiveResources`))
  (switch `/Game/Blueprints/Components/Lists/InventoryOwnerType` (`self.InventoryOwnerType`)
    (:`NewEnumerator0`
      (`self.CleanupGiver`)
      (return _itemstogive))
    (:`NewEnumerator1`
      (`self.ReplenishGiver`))))

(fn `TransactionReceiver`
  (params (ReceivedItems :type "Array of /Game/Blueprints/Components/Lists/Item Structure"))
  (`self.ReceiveResources` ReceivedItems))