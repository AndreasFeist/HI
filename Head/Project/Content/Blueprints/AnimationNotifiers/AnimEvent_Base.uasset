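; Base animation notify that spawns an AnimationEffect actor, set up to pick effects by ground surface and character part.
; A short vertical Visibility trace at the mesh's socket location reads the physical surface type, though the selected ID shown is always zero.
; On a hit, it looks up the character part in AnimNotifyInputs and spawns the effect with that ID only if an entry exists.
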(fn `ChooseEffect`
  (params (MeshComponent :type "SkeletalMeshComponent Object Reference") (SocetName :type Name))
  (returns (FoundOutput :type Boolean) (AnimNotifyOutput :type "/Game/Blueprints/AnimationNotifiers/Lists/AnimEvent_Outputs Structure") (SelectedID :type Integer))
  (locals (localSelectedID :type Integer))
  (bind _returnvalue (`SceneComponent.GetSocketLocation` MeshComponent SocetName))
  (bind (_value _returnvalue_2) (`BlueprintMapLibrary.Map_Find` (`self.AnimNotify_Inputs`) (`self.AnimNotifyCharPart`)))
  (bind (_outhit _returnvalue_3) (`KismetSystemLibrary.LineTraceSingle` (+ (0.0 0.0 50.0) _returnvalue) (- _returnvalue (0.0 0.0 50.0)) "TraceTypeQuery1"))
  (if _returnvalue_3
    (switch `EPhysicalSurface` (`PhysicalMaterial.SurfaceType` (`.PhysMat` (`GameplayStatics.BreakHitResult` _outhit)))
      (:`SurfaceType_Default`
        (set `local.localSelectedID` 0)
        (if _returnvalue_2
          (return true _value (`local.localSelectedID`))
          (else
            (return false (struct) 0)))))))

(fn `Received_Notify`
  (params (MeshComp :type "SkeletalMeshComponent Object Reference") (Animation :type "AnimSequenceBase Object Reference"))
  (returns (ReturnValue :type Boolean))
  (bind (_foundoutput _animnotifyoutput _selectedid) (`self.ChooseEffect` MeshComp))
  (if _foundoutput
    (`|SpawnActorFromClass` "/Game/Blueprints/AnimationNotifiers/AnimationEffect.AnimationEffect_C" (`self.AnimActorTransform`) "Undefined" "OverrideRootScale" null (struct) _selectedid null)
    (return true)
    (else
      (return false))))